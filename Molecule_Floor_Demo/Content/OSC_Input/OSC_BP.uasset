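; Actor that moves four primitive shapes from OSC skeleton-tracker data, one shape per tracked person.
; On BeginPlay it binds to its OSC receiver, then routes messages by address, matching the Neck joint of skeletons 0, 1, 3 and 4 to cube, cylinder, cone and sphere.
; The first and third floats are range-mapped with clamping to relative X and Y, with Z held fixed.
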(event `self.ReceiveBeginPlay`
  (add `OscReceiverComponent.OnOscReceived` (`self.OscReceiver`) (delegate `OSCRx`))
  (`KismetSystemLibrary.PrintString` "BP OSC Started"))

(event `OSCRx`
  (params (Address :type "Name (by ref)") (Data :type "Array of OscDataElemStruct Structure (by ref)") (SenderIp :type String))
  (bind (_output _value) (`OscFunctionLibrary.PopFloat` Data))
  (bind _returnvalue (`KismetMathLibrary.MakeVector` (`KismetMathLibrary.MapRangeClamped` _value -50.0 50.0 -1000.0 1000.0) (`KismetMathLibrary.MapRangeClamped` (`.Value` (`OscFunctionLibrary.PopFloat` (`OscFunctionLibrary.PopFloat` _output))) -50.0 50.0 -1000.0 1000.0) 50.0))
  (switch `name` Address
    (:`/skeletontracker/skeletons/0/Neck`
      (`SceneComponent.K2_SetRelativeLocation` (`self.Cube`) _returnvalue false false))
    (:`/skeletontracker/skeletons/1/Neck`
      (`SceneComponent.K2_SetRelativeLocation` (`self.Cylinder`) _returnvalue false false))
    (:`/skeletontracker/skeletons/4/Neck`
      (`SceneComponent.K2_SetRelativeLocation` (`self.Sphere`) _returnvalue false false))
    (:`/skeletontracker/skeletons/3/Neck`
      (`SceneComponent.K2_SetRelativeLocation` (`self.Cone`) _returnvalue false false))))

(fn `UserConstructionScript`)